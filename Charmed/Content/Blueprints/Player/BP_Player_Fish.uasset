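; Player fish pawn that swims by physics forces, collects charms on a trailing string and startles a kid on touching their legs.
; Input eases pitch and yaw onto Body; Object follows its position and velocity, and their yaw difference helps drive forward thrust.
; Tick also levels pitch, and obstacle or landscape hits push both components away.
; Charms attach to successive string bones, and collecting all changes the game controller's state.
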(event OnComponentHit(Object)
  (params (HitComponent :type Primitive%20Component%20Object%20Reference) (OtherActor :type Actor%20Object%20Reference) (OtherComp :type Primitive%20Component%20Object%20Reference) (NormalImpulse :type Vector :default "0, 0, 0") (Hit :type Hit%20Result%20Structure%20%28by%20ref%29))
  (if (or (== (Utilities|GetClass OtherActor) "/Script/Landscape.Landscape") (Utilities|Name|Equal(Name) (Utilities|Array|Get(acopy) (Variables|/Script/Engine.ActorComponent|GetComponentTags OtherComp)) "Obstacle"))
    (bind _returnvalue (Physics|GetPhysicsLinearVelocity (Variables|Default|GetBody) "None"))
    (Physics|AddForce (Variables|Default|GetBody) (* (.Normal (Collision|BreakHitResult Hit)) (* (Math|Vector|VectorLength _returnvalue) 1e+01)) "None" false)))

(event OnComponentBeginOverlap(Body)
  (params (OverlappedComponent :type Primitive%20Component%20Object%20Reference) (OtherActor :type Actor%20Object%20Reference) (OtherComp :type Primitive%20Component%20Object%20Reference) (OtherBodyIndex :type Integer) (bFromSweep :type Boolean) (SweepResult :type Hit%20Result%20Structure%20%28by%20ref%29))
  (switch name (Utilities|Array|Get(acopy) (Variables|/Script/Engine.ActorComponent|GetComponentTags OtherComp))
    (:Charm
      (CallFunction|PickUpCharm OtherComp))
    (:Kid
      (Variables|Objective|SetLegsTouched true)
      (Variables|Default|SetChildLegs OtherComp)
      (bind _asbp_objective_start_trigger (Utilities|Casting|CastToBP_ObjectiveStartTrigger OtherActor))
      (Default|StartleKid _asbp_objective_start_trigger)
      (Utilities|FlowControl|Delay (Variables|Default|GetResetTime))
      (Variables|Objective|SetLegsTouched false))))

(event EventTick
  (params (DeltaSeconds :type Float%20%28single-precision%29))
  (bind _pitchspeed (Variables|Movement|GetPitchSpeed))
  (bind _yawspeed (Variables|Movement|GetYawSpeed))
  (bind _object (Variables|Default|GetObject))
  (bind _body (Variables|Default|GetBody))
  (bind _returnvalue (Transformation|GetWorldLocation _body))
  (bind _returnvalue_2 (* DeltaSeconds _yawspeed))
  (bind _returnvalue_3 (* DeltaSeconds _pitchspeed))
  (bind _returnvalue_4 (Math|Rotator|MakeRotator 0.0 _returnvalue_3 _returnvalue_2))
  (Transformation|AddLocalRotation (Variables|Default|GetBody) _returnvalue_4 false false)
  (CallFunction|YawTurning _returnvalue_4)
  (CallFunction|PitchTurning)
  (CallFunction|LevelOut _object)
  (CallFunction|LevelOut _body)
  (CallFunction|ResetLinearVelocity)
  (CallFunction|ResetAngularVelocity)
  (if (Math|Vector|NotEqual(Vector) (Transformation|GetWorldLocation _object) _returnvalue 0.0)
    (Transformation|SetWorldLocation (Variables|Default|GetObject) _returnvalue false false))
  (bind _difference (CallFunction|GetYawDifference))
  (if (> _difference (+ (Variables|Movement|GetMaxTurn) 2.0))
    (Transformation|SetRelativeRotation (Variables|Default|GetObject) (Variables|/Script/Engine.SceneComponent|GetRelativeRotation _body) false false))
  (Rendering|SetVisibility (Variables|Default|GetString) (Variables|Objective|GetStarted) false))

(event EventBeginPlay
  (Class|SkeletalMeshComponent|SetAllBodiesBelowSimulatePhysics (Variables|Default|GetSkeletalMesh) (Variables|Bones|GetFishNeckBone) true true)
  (Class|SkeletalMeshComponent|SetAllBodiesBelowSimulatePhysics (Variables|Default|GetString) (Variables|Bones|GetStringBone) true true)
  (bind _asbp_game_controller (Utilities|Casting|CastToBP_GameController (Game|GetGameMode)))
  (Variables|References|SetGameModeReference _asbp_game_controller))

(event Input|AxisEvents|InputAxisMoveRight
  (params (AxisValue :type Float%20%28single-precision%29))
  (Variables|Movement|SetYawSpeed (Math|Interpolation|FInterpTo (Variables|Movement|GetYawSpeed) (* AxisValue (Variables|Movement|GetTurnSpeed)) (Utilities|Time|GetWorldDeltaSeconds) 2.0))
  (if (== AxisValue 0.0)
    (Variables|Movement|SetTurning false)
    (else
      (Variables|Movement|SetTurning true))))

(event Input|AxisEvents|InputAxisMoveUp
  (params (AxisValue :type Float%20%28single-precision%29))
  (Variables|Movement|SetPitchSpeed (Math|Interpolation|FInterpTo (Variables|Movement|GetPitchSpeed) (* (* AxisValue -1.0) (Variables|Movement|GetTurnSpeed)) (Utilities|Time|GetWorldDeltaSeconds) 2.0)))

(event Input|AxisEvents|InputAxisLookUp
  (params (AxisValue :type Float%20%28single-precision%29))
  (Pawn|Input|AddControllerPitchInput AxisValue))

(event Input|AxisEvents|InputAxisTurn
  (params (AxisValue :type Float%20%28single-precision%29))
  (Pawn|Input|AddControllerYawInput AxisValue))

(event Input|KeyboardEvents|Escape
  (params (Key :type Key%20Structure))
  (:Pressed
    (Game|QuitGame 0 "Quit")))

(fn ConstructionScript)

(fn LevelOut
  (params (Object :type Scene%20Component%20Object%20Reference))
  (bind _returnvalue (Transformation|GetWorldRotation Object))
  (bind _returnvalue_2 (Utilities|Time|GetWorldDeltaSeconds))
  (Transformation|SetWorldRotation Object (Math|Rotator|Lerp(Rotator) (Transformation|GetWorldRotation Object) (Math|Rotator|MakeRotator 0.0 (Math|Float|Lerp (.pitch _returnvalue) 0.0 (* _returnvalue_2 (LocalVariables|GetLevelSpeed))) (.yaw _returnvalue)) _returnvalue_2) false false))

(fn YawTurning
  (params (YawRotation :type Rotator))
  (bind _maxturn (Variables|Movement|GetMaxTurn))
  (bind _object (Variables|Default|GetObject))
  (bind _difference (CallFunction|GetYawDifference))
  (if (Variables|Movement|GetTurning)
    _
    (else
      (Variables|Movement|SetForce (Math|Float|Absolute(Float) _difference))))
  (bind _crossed (CallFunction|GetCross _difference (Variables|Movement|GetMaxTurn)))
  (if _crossed
    (bind _crossed_2 (CallFunction|GetCross _difference 0.5))
    (if _crossed_2
      (if (>= (Variables|Movement|GetForce) _maxturn)
        (Variables|Movement|SetForce _maxturn))
      (Physics|AddForce (Variables|Default|GetBody) (* (Math|Vector|GetForwardVector (Variables|Default|GetObject)) (* (Variables|Movement|GetForce) (Variables|Movement|GetForceRate))) "None" false))
    (else
      (Transformation|AddLocalRotation _object YawRotation false false)
      (if (Variables|Movement|GetTurning)
        (Physics|AddForce (Variables|Default|GetBody) (* (Math|Vector|GetForwardVector _object) (* (Variables|Movement|GetTurnForce) (Variables|Movement|GetForceRate))) "None" false)))))

(fn GetYawDifference
  (return (- (.yaw (Variables|/Script/Engine.SceneComponent|GetRelativeRotation (Variables|Default|GetObject))) (.yaw (Variables|/Script/Engine.SceneComponent|GetRelativeRotation (Variables|Default|GetBody))))))

(fn GetCross
  (params (Difference :type Float%20%28single-precision%29) (Offset :type Float%20%28single-precision%29))
  (return (and (> Difference (* Offset -1.0)) (< Difference Offset))))

(fn PitchTurning
  (bind _object (Variables|Default|GetObject))
  (bind _returnvalue (Transformation|GetWorldRotation _object))
  (if true
    (Transformation|SetWorldRotation _object (Math|Rotator|MakeRotator (.roll _returnvalue) (.pitch (Transformation|GetWorldRotation (Variables|Default|GetBody))) (.yaw _returnvalue)) false false)))

(fn PickUpCharm
  (params (Charm :type Scene%20Component%20Object%20Reference))
  (bind _string (Variables|Default|GetString))
  (Transformation|SetRelativeRotation Charm "90.000000, 0, 0" false false)
  (Transformation|AttachComponentToComponent Charm _string (Class|SkinnedMeshComponent|GetBoneName _string (+ (Variables|Default|GetStringStartIndex) (Variables|Objective|GetCharmsCollected))) "SnapToTarget" "KeepRelative" "KeepWorld" true)
  (bind _asstatic_mesh_component (Utilities|Casting|CastToStaticMeshComponent Charm))
  (Collision|SetCollisionObjectType _asstatic_mesh_component "ECC_PhysicsBody")
  (bind _output_get (Variables|Objective|SetCharmsCollected (+ (Variables|Objective|GetCharmsCollected) 1)))
  (if (== _output_get (Variables|Objective|GetNumCharms))
    (Variables|/Game/Blueprints/BP_GameController.BP_GameController_C|SetState (Variables|References|GetGameModeReference) "NewEnumerator2")))

(fn ResetLinearVelocity
  (bind _returnvalue (Physics|GetPhysicsLinearVelocity (Variables|Default|GetBody) "None"))
  (Class|PrimitiveComponent|SetAllPhysicsLinearVelocity (Variables|Default|GetObject) _returnvalue false))

(fn ResetAngularVelocity
  (bind _returnvalue (Class|PrimitiveComponent|GetPhysicsAngularVelocityinRadians (Variables|Default|GetBody) "None"))
  (Class|PrimitiveComponent|SetAllPhysicsAngularVelocityinRadians (Variables|Default|GetObject) _returnvalue false))

(fn GlowAllCharms)