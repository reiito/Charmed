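; Player shark pawn that swims with physics forces, steered by a head that leads the body, with physics simulated on the fish's bones below a set bone.
; Move inputs ease pitch and yaw speeds that rotate FishHead each tick; the body copies head pitch, and both gradually level out.
; Head-to-body yaw difference drives thrust and damping: within TurnMax it can trigger a forward push, beyond it the body turns with decaying force.
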(event EventBeginPlay
  (Class|SkeletalMeshComponent|SetAllBodiesBelowSimulatePhysics (Variables|Default|GetFish) (Variables|Default|GetNextBone) true true))

(event EventTick
  (params (DeltaSeconds :type Float%20%28single-precision%29))
  (bind _pitchspeed (Variables|Default|GetPitchSpeed))
  (bind _yawspeed (Variables|Default|GetYawSpeed))
  (bind _returnvalue (* DeltaSeconds _yawspeed))
  (bind _returnvalue_2 (* DeltaSeconds _pitchspeed))
  (bind _returnvalue_3 (Math|Rotator|MakeRotator 0.0 _returnvalue_2 _returnvalue))
  (Transformation|AddLocalRotation (Variables|Default|GetFishHead) _returnvalue_3 false false)
  (CallFunction|YawTurning _returnvalue_3)
  (CallFunction|PitchTurning)
  (CallFunction|Straighten (Variables|Default|GetStaticMesh))
  (CallFunction|Straighten (Variables|Default|GetFishHead)))

(event Input|AxisEvents|InputAxisMoveRight
  (params (AxisValue :type Float%20%28single-precision%29))
  (Variables|Default|SetYawSpeed (Math|Interpolation|FInterpTo (Variables|Default|GetYawSpeed) (* AxisValue (Variables|Default|GetTurnSpeed)) (Utilities|Time|GetWorldDeltaSeconds) 2.0))
  (if (== AxisValue 0.0)
    (Variables|Default|SetTurning false)
    (else
      (Variables|Default|SetTurning true))))

(event Input|AxisEvents|InputAxisMoveUp
  (params (AxisValue :type Float%20%28single-precision%29))
  (Variables|Default|SetPitchSpeed (Math|Interpolation|FInterpTo (Variables|Default|GetPitchSpeed) (* (* AxisValue -1.0) (Variables|Default|GetTurnSpeed)) (Utilities|Time|GetWorldDeltaSeconds) 2.0)))

(event Input|AxisEvents|InputAxisLookUp
  (params (AxisValue :type Float%20%28single-precision%29))
  (Pawn|Input|AddControllerPitchInput AxisValue))

(event Input|AxisEvents|InputAxisTurn
  (params (AxisValue :type Float%20%28single-precision%29))
  (Pawn|Input|AddControllerYawInput AxisValue))

(fn ConstructionScript)

(fn GetYawDifference
  (return (- (.yaw (Variables|/Script/Engine.SceneComponent|GetRelativeRotation (Variables|Default|GetFishHead))) (.yaw (Variables|/Script/Engine.SceneComponent|GetRelativeRotation (Variables|Default|GetStaticMesh))))))

(fn GetPitchDifference
  (return (- (.pitch (Variables|/Script/Engine.SceneComponent|GetRelativeRotation (Variables|Default|GetFishHead))) (.pitch (Variables|/Script/Engine.SceneComponent|GetRelativeRotation (Variables|Default|GetStaticMesh))))))

(fn YawTurning
  (params (Rotation :type Rotator))
  (bind _fishhead (Variables|Default|GetFishHead))
  (bind _turnmax (Variables|Default|GetTurnMax))
  (bind _staticmesh (Variables|Default|GetStaticMesh))
  (bind _difference (CallFunction|GetYawDifference))
  (if (and (> _difference (* _turnmax -1.0)) (< _difference _turnmax))
    (CallFunction|ForcePush _difference)
    (else
      (Transformation|AddLocalRotation _staticmesh Rotation false false)
      (Class|PrimitiveComponent|SetLinearDamping _fishhead 0.5)
      (Physics|AddForce _fishhead (* (Math|Vector|GetForwardVector _staticmesh) (Variables|Default|GetTurnForce)) "None" false)
      (Variables|Default|SetTurnForce (Math|Float|Lerp (Variables|Default|GetTurnForce) 0.0 (Utilities|Time|GetWorldDeltaSeconds))))))

(fn PitchTurning
  (bind _staticmesh (Variables|Default|GetStaticMesh))
  (bind _returnvalue (Transformation|GetWorldRotation _staticmesh))
  (Transformation|SetWorldRotation _staticmesh (Math|Rotator|MakeRotator (.roll _returnvalue) (.pitch (Transformation|GetWorldRotation (Variables|Default|GetFishHead))) (.yaw _returnvalue)) false false))

(fn ForcePush
  (params (Difference :type Float%20%28single-precision%29))
  (bind _staticmesh (Variables|Default|GetStaticMesh))
  (bind _staticmesh_2 (Variables|Default|GetStaticMesh))
  (if (Variables|Default|GetTurning)
    (Class|PrimitiveComponent|SetLinearDamping _staticmesh_2 0.1)
    (else
      (Class|PrimitiveComponent|SetLinearDamping _staticmesh_2 0.15)
      (Variables|Default|SetForce (Math|Float|Absolute(Float) (/ Difference (Variables|Default|GetForceRate))))))
  (if (Math|Float|NearlyEqual(Float) Difference (Variables|Default|GetTurnOffset) 1.0)
    (Physics|AddForce _staticmesh (* (Math|Vector|GetForwardVector _staticmesh) (Variables|Default|GetForce)) "None" false)))

(fn Straighten
  (params (Mesh :type Static%20Mesh%20Component%20Object%20Reference))
  (bind _returnvalue (Transformation|GetWorldRotation Mesh))
  (bind _returnvalue_2 (Utilities|Time|GetWorldDeltaSeconds))
  (Transformation|SetWorldRotation Mesh (Math|Rotator|Lerp(Rotator) (Transformation|GetWorldRotation Mesh) (Math|Rotator|MakeRotator 0.0 (Math|Float|Lerp (.pitch _returnvalue) 0.0 (* _returnvalue_2 2.0)) (.yaw _returnvalue)) _returnvalue_2) false false))