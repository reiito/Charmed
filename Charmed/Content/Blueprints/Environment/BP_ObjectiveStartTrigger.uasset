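; Objective trigger for a child NPC's bracelet quest, given and completed when the fish player overlaps its capsule.
; In ROAMING, overlap places five charms and plays typewriter HUD dialogue, then sets LOOKING unless the player touched the legs, which cuts dialogue short.
; In COLLECTED, charms glow, and overlap destroys them, thanks the fish and sets DONE.
; Tick lerps the legs upward when touched or finished, otherwise back to their start.
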(event OnComponentBeginOverlap(Capsule)
  (params (OverlappedComponent :type Primitive%20Component%20Object%20Reference) (OtherActor :type Actor%20Object%20Reference) (OtherComp :type Primitive%20Component%20Object%20Reference) (OtherBodyIndex :type Integer) (bFromSweep :type Boolean) (SweepResult :type Hit%20Result%20Structure%20%28by%20ref%29))
  (if (== OtherActor (Variables|References|GetPlayerReference))
    (Rendering|Components|TextRender|SetText (Variables|References|GetHUDText) "")
    (switch Utilities|FlowControl|Switch|SwitchonENUM_States (Variables|/Game/Blueprints/BP_GameController.BP_GameController_C|GetState (Variables|References|GetGameModeReference))
      (:NewEnumerator0
        (CallFunction|StartObjective))
      (:NewEnumerator2
        (Variables|/Game/Blueprints/Player/BP_Player_Fish.BP_Player_Fish_C|SetStarted (Variables|References|GetPlayerReference) false)
        (CallFunction|EndObjective)))
    (Variables|/Game/Blueprints/Player/BP_Player_Fish.BP_Player_Fish_C|SetTriggered (Variables|References|GetPlayerReference) true)))

(event Custom|StartObjectiveText
  (bind _playerreference (Variables|References|GetPlayerReference))
  (bind _legstouched (Variables|/Game/Blueprints/Player/BP_Player_Fish.BP_Player_Fish_C|GetLegsTouched _playerreference))
  (bind _arrayelement (Utilities|DelayedforEachLoop (Variables|Default|GetDialogue) :!label _label)
    (:LoopBody
      (Utilities|ScrollText (Variables|References|GetHUDText) _arrayelement (Variables|Default|GetTypeSpeed) _legstouched)
      (if _legstouched
        (goto _label NextBody)
        (else
          (Utilities|FlowControl|Delay (Variables|Default|GetTalkSpeed))
          (goto _label NextBody))))
    (:Completed
      (if _legstouched
        (Variables|/Game/Blueprints/BP_GameController.BP_GameController_C|SetState (Variables|References|GetGameModeReference) "NewEnumerator0")
        (Variables|/Game/Blueprints/Player/BP_Player_Fish.BP_Player_Fish_C|SetStarted (Variables|References|GetPlayerReference) false)
        (Utilities|FlowControl|Delay 5.0)
        (else
          (Variables|/Game/Blueprints/BP_GameController.BP_GameController_C|SetState (Variables|References|GetGameModeReference) "NewEnumerator1")))
      (Variables|Booleans|SetStartDone true))))

(event Custom|StartObjective
  (Variables|/Game/Blueprints/Player/BP_Player_Fish.BP_Player_Fish_C|SetStarted (Variables|References|GetPlayerReference) true)
  (CallFunction|SpawnObjectives)
  (CallFunction|StartObjectiveText))

(event Custom|StartleKid
  (bind _playerreference (Variables|References|GetPlayerReference))
  (if (Variables|/Game/Blueprints/Player/BP_Player_Fish.BP_Player_Fish_C|GetLegsTouched _playerreference)
    (Utilities|FlowControl|Delay 0.5)
    (Variables|/Game/Blueprints/Player/BP_Player_Fish.BP_Player_Fish_C|SetTriggered _playerreference true)
    (Utilities|ScrollText (Variables|References|GetHUDText) "Child: Ah! What was that?!" (Variables|Default|GetTypeSpeed) false)
    (Utilities|FlowControl|Delay (Variables|Default|GetTalkSpeed)))
  (Variables|/Game/Blueprints/Player/BP_Player_Fish.BP_Player_Fish_C|SetTriggered (Variables|References|GetPlayerReference) false))

(event Custom|EndObjective
  (bind _hudtext (Variables|References|GetHUDText))
  (Utilities|FlowControl|Sequence
    (:then_0
      (for _array_element (Variables|Default|GetCharmObjects)
        (Components|DestroyComponent _array_element)
        (Variables|Booleans|SetObjectiveComplete true)
        (Variables|/Game/Blueprints/BP_GameController.BP_GameController_C|SetState (Variables|References|GetGameModeReference) "NewEnumerator3")))
    (:then_1
      (Utilities|ScrollText _hudtext "Child: Wow! That fish just gave me my braclet!" (Variables|Default|GetTypeSpeed) false)
      (Utilities|FlowControl|Delay (Variables|Default|GetTalkSpeed))
      (Utilities|ScrollText _hudtext "Child: Thanks little one!" (Variables|Default|GetTypeSpeed) false)
      (Utilities|FlowControl|Delay (Variables|Default|GetTalkSpeed))
      (Variables|Booleans|SetEndDone true))))

(event EventBeginPlay
  (bind _asbp_game_controller (Utilities|Casting|CastToBP_GameController (Game|GetGameMode)))
  (bind _output_get (Variables|References|SetGameModeReference _asbp_game_controller))
  (bind _asbp_player_fish (Utilities|Casting|CastToBP_Player_Fish (Game|Player|GetPlayerPawn 0)))
  (Variables|References|SetPlayerReference _asbp_player_fish)
  (Variables|References|SetHUDText (Variables|/Game/Blueprints/HUD/BP_ChildText.BP_ChildText_C|GetObjectiveDialogue (Variables|/Game/Blueprints/BP_GameController.BP_GameController_C|GetHUDReference _output_get)))
  (Variables|Default|SetLegLocation (Transformation|GetWorldLocation (Variables|Default|GetLegs))))

(event EventTick
  (params (DeltaSeconds :type Float%20%28single-precision%29))
  (if (Utilities|Enum|Equal(Enum) (Variables|/Game/Blueprints/BP_GameController.BP_GameController_C|GetState (Variables|References|GetGameModeReference)) "NewEnumerator2")
    (for _array_element (Variables|Default|GetCharmObjects)
      (Rendering|Material|SetMaterial _array_element 0 "/Game/Materials/Charms/M_CharmGlow.M_CharmGlow")
      (if (Variables|/Game/Blueprints/Player/BP_Player_Fish.BP_Player_Fish_C|GetLegsTouched (Variables|References|GetPlayerReference))
        (CallFunction|MoveLegs)
        (else
          (CallFunction|ResetLegs)))
      (if (Variables|Booleans|GetObjectiveComplete)
        (CallFunction|MoveLegs)
        (if (Variables|Booleans|GetEndDone)
          (Variables|Booleans|SetEndDone false)
          (Variables|/Game/Blueprints/Player/BP_Player_Fish.BP_Player_Fish_C|SetTriggered (Variables|References|GetPlayerReference) false))
        (elif (Variables|Booleans|GetStartDone)
          (Variables|Booleans|SetStartDone false)
          (Variables|/Game/Blueprints/Player/BP_Player_Fish.BP_Player_Fish_C|SetTriggered (Variables|References|GetPlayerReference) false))))
    (else
      (if (Variables|/Game/Blueprints/Player/BP_Player_Fish.BP_Player_Fish_C|GetLegsTouched (Variables|References|GetPlayerReference))
        (CallFunction|MoveLegs)
        (else
          (CallFunction|ResetLegs)))
      (if (Variables|Booleans|GetObjectiveComplete)
        (CallFunction|MoveLegs)
        (if (Variables|Booleans|GetEndDone)
          (Variables|Booleans|SetEndDone false)
          (Variables|/Game/Blueprints/Player/BP_Player_Fish.BP_Player_Fish_C|SetTriggered (Variables|References|GetPlayerReference) false))
        (elif (Variables|Booleans|GetStartDone)
          (Variables|Booleans|SetStartDone false)
          (Variables|/Game/Blueprints/Player/BP_Player_Fish.BP_Player_Fish_C|SetTriggered (Variables|References|GetPlayerReference) false))))))

(fn ConstructionScript)

(fn SpawnObjectives
  (bind _output_get (Variables|Default|SetCharmObjects (Utilities|Array|MakeArray (Variables|Default|GetCharm1) (Variables|Default|GetCharm2) (Variables|Default|GetCharm3) (Variables|Default|GetCharm4) (Variables|Default|GetCharm5))))
  (for (_array_element _array_index) _output_get
    (Rendering|SetVisibility _array_element true false)
    (Transformation|SetWorldLocation _array_element (Utilities|Array|Get(acopy) (LocalVariables|GetCharmLocations) _array_index) false false)))

(fn MoveLegs
  (bind _legs (Variables|Default|GetLegs))
  (bind _returnvalue (Transformation|GetWorldLocation _legs))
  (Transformation|SetWorldLocation _legs (Math|Vector|Lerp(Vector) (Transformation|GetWorldLocation _legs) (Math|Vector|MakeVector (.x _returnvalue) (.y _returnvalue) (LocalVariables|GetRetreatHeight)) (Utilities|Time|GetWorldDeltaSeconds)) false false))

(fn ResetLegs
  (bind _legs (Variables|Default|GetLegs))
  (Transformation|SetWorldLocation _legs (Math|Vector|Lerp(Vector) (Transformation|GetWorldLocation _legs) (Variables|Default|GetLegLocation) (* (Utilities|Time|GetWorldDeltaSeconds) (LocalVariables|GetSpeed))) false false))